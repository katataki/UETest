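; BP_EmojiSphere is an actor whose sphere component gets pushed away from a shared light point in the horizontal plane.
; Each tick, Fluence reads LightPoint from the MPC_Emoji material parameter collection and sets the sphere's relative offset along the 2D direction away from it.
; The offset scales with Strength and fades linearly to zero at MaxDistance, measured from the sphere's current, already displaced world position.
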(event `self.ReceiveTick`
  (params (DeltaSeconds :type "Float (single-precision)"))
  (`self.Fluence`))

(fn `Fluence`
  (locals (LightPos :type "Vector Structure" :default (0.0 0.0 0.0)))
  (bind _returnvalue (`SceneComponent.K2_GetComponentLocation` (`self.Sphere`)))
  (bind _returnvalue_2 (`KismetMaterialLibrary.GetVectorParameterValue` "/Game/EmojiInteraction/Materials/MPC_Emoji.MPC_Emoji" "LightPoint"))
  (bind _output_get (set `local.LightPos` (`KismetMathLibrary.Conv_LinearColorToVector` _returnvalue_2)))
  (`SceneComponent.K2_SetRelativeLocation` (`self.Sphere`) (* (`KismetMathLibrary.Vector_Normal2D` (- _returnvalue (`local.LightPos`))) (* (- 1.0 (`KismetMathLibrary.FClamp` (/ (`KismetMathLibrary.Vector_Distance2D` _output_get _returnvalue) (`self.MaxDistance`)))) (`self.Strength`))) false false))

(fn `UserConstructionScript`)